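; Default unit class for a tower defense (TD) game, holding an array of upgradeable stats indexed by status ID.
; Leveling up rebuilds the stat struct with one more level and a value increase scaled by the current level and a correction factor.
; The level check returns the current level and the next upgrade cost, summed from per-level terms rounded to hundreds.
; Click and release functions are empty stubs, and cursor hover on the cylinder only prints a debug string.
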(event OnBeginCursorOver(Cylinder)
  (params (TouchedComponent :type Primitive%20Component%20Object%20Reference))
  (Development|PrintString "んご"))

(event EventBeginPlay)

(fn ConstructionScript)

(fn FuncLevelUpStatus
  (params (StatusId :type Integer))
  (Utilities|Array|SetArrayElem (Variables|Default|GetStatus) StatusId (Utilities|Struct|MakeTD_StatusDetail (.Name (Utilities|Struct|BreakTD_StatusDetail (Utilities|Array|Get(acopy) (Variables|Default|GetStatus) StatusId))) (.Id (Utilities|Struct|BreakTD_StatusDetail (Utilities|Array|Get(acopy) (Variables|Default|GetStatus) StatusId))) (+ (.Val (Utilities|Struct|BreakTD_StatusDetail (Utilities|Array|Get(acopy) (Variables|Default|GetStatus) StatusId))) (Math|Float|Floor (* (.LevelUpVal (Utilities|Struct|BreakTD_StatusDetail (Utilities|Array|Get(acopy) (Variables|Default|GetStatus) StatusId))) (* (.Level (Utilities|Struct|BreakTD_StatusDetail (Utilities|Array|Get(acopy) (Variables|Default|GetStatus) StatusId))) (.LevelUpVal_correct (Utilities|Struct|BreakTD_StatusDetail (Utilities|Array|Get(acopy) (Variables|Default|GetStatus) StatusId))))))) (+ (.Level (Utilities|Struct|BreakTD_StatusDetail (Utilities|Array|Get(acopy) (Variables|Default|GetStatus) StatusId))) 1) (.LevelUpMoney (Utilities|Struct|BreakTD_StatusDetail (Utilities|Array|Get(acopy) (Variables|Default|GetStatus) StatusId))) (.LevelUpMoney_correct (Utilities|Struct|BreakTD_StatusDetail (Utilities|Array|Get(acopy) (Variables|Default|GetStatus) StatusId))) (.LevelUpVal (Utilities|Struct|BreakTD_StatusDetail (Utilities|Array|Get(acopy) (Variables|Default|GetStatus) StatusId))) (.LevelUpVal_correct (Utilities|Struct|BreakTD_StatusDetail (Utilities|Array|Get(acopy) (Variables|Default|GetStatus) StatusId)))))
  (bind _output_get (Variables|Default|SetStatus (Variables|Default|GetStatus)))
  (return _output_get))

(fn FuncStatusLevelCheck
  (params (Status%20Id :type Integer))
  (bind _status (Variables|Default|GetStatus))
  (bind _item (Utilities|Array|Get(acopy) _status Status%20Id))
  (bind (_name _id _val _level _levelupmoney _levelupmoney_correct) (Utilities|Struct|BreakTD_StatusDetail _item))
  (for _index (range 1 _level)
    (bind _output_get (LocalVariables|Setnum (+ (LocalVariables|Getnum) (Math|Float|Truncate (* (Math|Float|Round (/ (* (* _index _levelupmoney) _levelupmoney_correct) 1e+02)) 1e+02))))))
  (return _level _output_get))

(fn FuncClickEvent)

(fn FuncReleaseEvent)