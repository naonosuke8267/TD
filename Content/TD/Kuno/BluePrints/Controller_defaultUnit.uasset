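; Controller for the default unit in a TD game, pacing how often the controlled unit acts.
; Each Tick increments a behavior counter until it exceeds the unit's status entry 3, then resets it and calls Func_Action, making the interval frame-based.
; Status is read by casting the controlled pawn to Class_defaultUnit and indexing its Status.
; Func_Action is a placeholder that only prints "Action".
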(event `self.ReceiveTick`
  (params (DeltaSeconds :type "Float (single-precision)"))
  (bind _cnt_behavior (`self.cnt_Behavior`))
  (if (> _cnt_behavior (`.Val_18_047C3F3F4197AAA8E382A98AE98CAF25` (break `/Game/TD/Kuno/Etc/TD_StatusDetail` (`self.Func_GetUnitStatus` 3))))
    (set `self.cnt_Behavior` 0)
    (`self.Func_Action`)
    (else
      (`/Engine/EditorBlueprintResources/StandardMacros.IncrementInt` _cnt_behavior))))

(fn `Func_Action`
  (`KismetSystemLibrary.PrintString` "Action"))

(fn `Func_GetUnitStatus`
  (params (`Status Id` :type Integer))
  (returns (`Return Status` :type "/Game/TD/Kuno/Etc/TD_StatusDetail Structure"))
  (return (`KismetArrayLibrary.Array_Get` (`/Game/TD/Kuno/BluePrints/Class_defaultUnit.Status` (cast `/Game/TD/Kuno/BluePrints/Class_defaultUnit` (`self.K2_GetPawn`) :!pure true)) `Status Id`)))

(fn `UserConstructionScript`)